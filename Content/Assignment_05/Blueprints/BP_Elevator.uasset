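; BP_Elevator is a platform that rises when a BP_Ball enters its trigger box and lowers when the ball leaves.
; On overlap it swaps the platform material to a green light, waits a delay, then plays the OpenDoor timeline to lerp the platform's relative location from zero to UPLocation.
; On end overlap it switches to a red material and reverses the timeline after the same delay.
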(event `self.Box.OnComponentBeginOverlap`
  (params (OverlappedComponent :type "PrimitiveComponent Object Reference") (OtherActor :type "Actor Object Reference") (OtherComp :type "PrimitiveComponent Object Reference") (OtherBodyIndex :type Integer) (bFromSweep :type Boolean) (SweepResult :type "HitResult Structure (by ref)"))
  (cast `/Game/Assignment_05/Blueprints/BP_Ball` OtherActor)
  (`PrimitiveComponent.SetMaterial` (`self.Platform`) 0 "/Game/SuperGrid/TutorialLevel/MaterialInstances/M_Tut_LightG.M_Tut_LightG")
  (`KismetSystemLibrary.Delay` (`self.Delay`))
  (bind (_direction _newtrack_0) (`Timeline|OpenDoor` :!label _label)
    (:`Update`
      (`SceneComponent.K2_SetRelativeLocation` (`self.Platform`) (`KismetMathLibrary.VLerp` (0.0 0.0 0.0) (`self.UPLocation`) _newtrack_0) false false))))

(event `self.Box.OnComponentEndOverlap`
  (params (OverlappedComponent :type "PrimitiveComponent Object Reference") (OtherActor :type "Actor Object Reference") (OtherComp :type "PrimitiveComponent Object Reference") (OtherBodyIndex :type Integer))
  (cast `/Game/Assignment_05/Blueprints/BP_Ball` OtherActor)
  (`PrimitiveComponent.SetMaterial` (`self.Platform`) 0 "/Game/SuperGrid/TutorialLevel/MaterialInstances/M_Tut_Red1.M_Tut_Red1")
  (`KismetSystemLibrary.Delay` (`self.Delay`))
  (goto _label :!via `Reverse`))

(fn `UserConstructionScript`)