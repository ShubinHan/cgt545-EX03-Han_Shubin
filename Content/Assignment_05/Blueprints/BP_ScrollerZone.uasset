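; BP_ScrollerZone is a trigger volume that switches a BP_Ball into scroll control and changes the player's camera view.
; On box overlap, it blends player 0's view to itself, enables the ball's ScrollControll flag and sets its MoveTarget to the zone's Arrow.
; Leaving blends back to the player pawn and clears both ball values.
; The view blends run for any overlapping actor, before the BP_Ball cast.
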(event `self.Box.OnComponentBeginOverlap`
  (params (OverlappedComponent :type "PrimitiveComponent Object Reference") (OtherActor :type "Actor Object Reference") (OtherComp :type "PrimitiveComponent Object Reference") (OtherBodyIndex :type Integer) (bFromSweep :type Boolean) (SweepResult :type "HitResult Structure (by ref)"))
  (`PlayerController.SetViewTargetWithBlend` (`GameplayStatics.GetPlayerController` 0) self (`self.Blend Time_in`) "VTBlend_Linear" 0.0 true)
  (bind _asbp_ball (cast `/Game/Assignment_05/Blueprints/BP_Ball` OtherActor))
  (set `/Game/Assignment_05/Blueprints/BP_Ball.ScrollControll` true _asbp_ball)
  (set `/Game/Assignment_05/Blueprints/BP_Ball.MoveTarget` (`self.Arrow`) _asbp_ball))

(event `self.Box.OnComponentEndOverlap`
  (params (OverlappedComponent :type "PrimitiveComponent Object Reference") (OtherActor :type "Actor Object Reference") (OtherComp :type "PrimitiveComponent Object Reference") (OtherBodyIndex :type Integer))
  (`PlayerController.SetViewTargetWithBlend` (`GameplayStatics.GetPlayerController` 0) (`GameplayStatics.GetPlayerPawn` 0) (`self.Blend Time_out`) "VTBlend_Linear" 0.0 true)
  (bind _asbp_ball (cast `/Game/Assignment_05/Blueprints/BP_Ball` OtherActor))
  (set `/Game/Assignment_05/Blueprints/BP_Ball.ScrollControll` false _asbp_ball)
  (set `/Game/Assignment_05/Blueprints/BP_Ball.MoveTarget` null _asbp_ball))

(fn `UserConstructionScript`)