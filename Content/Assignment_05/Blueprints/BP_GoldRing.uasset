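; BP_GoldRing is a spinning collectible ring that awards score when a BP_Ball overlaps it.
; Tick increments the actor's yaw by a fixed amount each frame, so rotation speed depends on frame rate.
; On Sphere1 overlap, a CanScore flag ensures a single award through the ball's UpdateScore.
; The ring then plays ACoin and destroys itself after a delay.
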(event `self.ReceiveTick`
  (params (DeltaSeconds :type "Float (single-precision)"))
  (bind (_returnvalue_roll _returnvalue_pitch _returnvalue_yaw) (`KismetMathLibrary.BreakRotator` (`self.K2_GetActorRotation`)))
  (`self.K2_SetActorRotation` (`KismetMathLibrary.MakeRotator` _returnvalue_roll _returnvalue_pitch (+ _returnvalue_yaw 1.0))))

(event `self.Sphere1.OnComponentBeginOverlap`
  (params (OverlappedComponent :type "PrimitiveComponent Object Reference") (OtherActor :type "Actor Object Reference") (OtherComp :type "PrimitiveComponent Object Reference") (OtherBodyIndex :type Integer) (bFromSweep :type Boolean) (SweepResult :type "HitResult Structure (by ref)"))
  (bind _asbp_ball (cast `/Game/Assignment_05/Blueprints/BP_Ball` OtherActor))
  (if (`self.CanScore`)
    (set `self.CanScore` false)
    (`/Game/Assignment_05/Blueprints/BP_Ball.Update Score` _asbp_ball)
    (`AudioComponent.Play` (`self.A_Coin`) 0.0)
    (`KismetSystemLibrary.Delay` (`self.Delay`))
    (`self.K2_DestroyActor`)))

(fn `UserConstructionScript`)